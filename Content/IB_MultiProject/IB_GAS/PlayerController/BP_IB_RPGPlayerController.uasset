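; Player controller Blueprint for the IB GAS RPG, used mainly as a debug-key test harness.
; Keys display the quest log, connect to a localhost server, and set a dynamic projectile or sword through gameplay tags and ability levels.
; Another key calls the Serverspawncannon event, which spawns a cannon owned by this controller.
; Inventory widget toggle and item-adding nodes remain but are disconnected.
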(event Custom|serverspawncannon
  (params (NewParam :type Player%20Controller%20Object%20Reference))
  (Actor|GetActorOfClass "/Game/IB_MultiProject/Cannon/BP_CannonSpawnManager.BP_CannonSpawnManager_C")
  (Game|SpawnActorfromClass "/Game/IB_MultiProject/Cannon/BP_Cannon.BP_Cannon_C" (Math|Transform|MakeTransform "0, 0, 0" "0, 0, 0" "1.000000,1.000000,1.000000") "AlwaysSpawn" "MultiplyWithRoot" NewParam 0))

(event EventTick
  (params (DeltaSeconds :type Float%20%28single-precision%29)))

(event Input|KeyboardEvents|DebugKeyTab
  (params (Key :type Key%20Structure :default "None") (ActionValue :type Input%20Action%20Value%20Structure)))

(event Input|KeyboardEvents|DebugKey1
  (params (Key :type Key%20Structure :default "None") (ActionValue :type Input%20Action%20Value%20Structure)))

(event Input|KeyboardEvents|DebugKey3
  (params (Key :type Key%20Structure :default "None") (ActionValue :type Input%20Action%20Value%20Structure)))

(event Input|KeyboardEvents|DebugKey0
  (params (Key :type Key%20Structure :default "None") (ActionValue :type Input%20Action%20Value%20Structure))
  (:Pressed
    (Game|OpenLevel(byName) "127.0.0.1")))

(event Input|KeyboardEvents|DebugKey3
  (params (Key :type Key%20Structure :default "None") (ActionValue :type Input%20Action%20Value%20Structure))
  (:Pressed
    (bind _output_get (Variables|Default|SetRandomAbilityLevel (Math|Random|RandomIntegerinRange 25 25)))
    (Class|RPGAbilitySystemInterface|SetDynamicProjectile (GameplayTags|MakeLiteralGameplayTag "(TagName=\"Projectile.Basic.Type1\")") _output_get)
    (Development|PrintString (Utilities|String|ToString(Text) (Utilities|Text|FormatText " AbilityLevel : { }" (Utilities|Text|ToText(Integer) _output_get))))))

(event Input|KeyboardEvents|DebugKey4
  (params (Key :type Key%20Structure :default "None") (ActionValue :type Input%20Action%20Value%20Structure))
  (:Pressed
    (Class|RPGAbilitySystemInterface|SetDynamicWeapon (GameplayTags|MakeLiteralGameplayTag "(TagName=\"Item.Equippable.Weapon.Sword\")") 1)))

(event Input|KeyboardEvents|DebugKeyQ
  (params (Key :type Key%20Structure :default "None") (ActionValue :type Input%20Action%20Value%20Structure))
  (:Pressed
    (Class|IBRPGPlayerController|DisplayQuestLog)))

(event Input|KeyboardEvents|DebugKey5
  (params (Key :type Key%20Structure :default "None") (ActionValue :type Input%20Action%20Value%20Structure)))

(event Input|KeyboardEvents|DebugKey2
  (params (Key :type Key%20Structure :default "None") (ActionValue :type Input%20Action%20Value%20Structure)))

(event Input|KeyboardEvents|DebugKey7
  (params (Key :type Key%20Structure :default "None") (ActionValue :type Input%20Action%20Value%20Structure))
  (:Pressed
    (CallFunction|Serverspawncannon self)))

(fn ConstructionScript)