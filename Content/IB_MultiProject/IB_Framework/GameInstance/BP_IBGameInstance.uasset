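; Game instance Blueprint for a multiplayer game that creates dedicated-server sessions for the lobby and for dungeons.
; Two custom events use Advanced Sessions, publishing server name and map name as extra session settings.
; The dungeon event takes its map name and port as inputs, also advertises the port, and allows four public connections.
; Both events only print the success or failure result.
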(event EventCreateLobbySession
  (|AdvancedSession (Utilities|Array|MakeArray (Class|AdvancedSessionsLibrary|MakeLiteralSessionPropertyString "SteamServerName" "TheFlyingKnightServer") (Class|AdvancedSessionsLibrary|MakeLiteralSessionPropertyString "MAPNAME" "L_Lobby")) (Game|GetPlayerController 0) 100 0 false true true true true false false false true false true
    (:OnSuccess
      (Development|PrintString "ServerSuccessfully started"))
    (:OnFailure
      (Development|PrintString "Server did not started"))))

(event EventCreateDungeonSession
  (params (DungeonName :type String) (GeneratedPort :type Integer%20%28by%20ref%29))
  (|AdvancedSession (Utilities|Array|MakeArray (Class|AdvancedSessionsLibrary|MakeLiteralSessionPropertyString "SteamServerName" "TheFlyingKnightServer") (Class|AdvancedSessionsLibrary|MakeLiteralSessionPropertyString "MAPNAME" DungeonName) (Class|AdvancedSessionsLibrary|MakeLiteralSessionPropertyInt "PORT" GeneratedPort)) (Game|GetPlayerController 0) 4 0 false true true true true false false false true false true
    (:OnSuccess
      (Development|PrintString "Dungeon ServerSuccessfully started"))
    (:OnFailure
      (Development|PrintString "Dungeon Server did not started"))))